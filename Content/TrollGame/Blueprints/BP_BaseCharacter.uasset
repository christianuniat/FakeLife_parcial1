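; BP_BaseCharacter is a player character with look and movement controls that detects whether the wall it faces is solid or fake.
; Enhanced Input actions drive controller yaw and pitch, plus forward and sideways movement relative to control yaw.
; Every Tick, a debug-drawn Visibility line trace runs a short distance from the camera.
; Hit actors implementing BPI_WallInteractions report their wall type, which sets the boolean sent back to toggle their state.
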(event `EnhancedInput|/Game/TrollGame/Blueprints/Inputs/IA_Look`
  (params (ActionValue :type "Vector2D Structure") (ElapsedSeconds :type "Float (double-precision)") (TriggeredSeconds :type "Float (double-precision)") (InputAction :type "InputAction Object Reference" :default "/Game/TrollGame/Blueprints/Inputs/IA_Look.IA_Look"))
  ; Controla la camara de el personaje
  (:`Triggered`
    (`self.AddControllerYawInput` ActionValue_X)
    (`self.AddControllerPitchInput` ActionValue_Y)))

(event `EnhancedInput|/Game/TrollGame/Blueprints/Inputs/IA_MoveForward`
  (params (ActionValue :type "Float (double-precision)") (ElapsedSeconds :type "Float (double-precision)") (TriggeredSeconds :type "Float (double-precision)") (InputAction :type "InputAction Object Reference" :default "/Game/TrollGame/Blueprints/Inputs/IA_MoveForward.IA_MoveForward"))
  (bind (_returnvalue_roll _returnvalue_pitch _returnvalue_yaw) (`KismetMathLibrary.BreakRotator` (`self.GetControlRotation`)))
  ; Control de movimiento frontal
  (:`Triggered`
    (`self.AddMovementInput` (`KismetMathLibrary.GetForwardVector` (`KismetMathLibrary.MakeRotator` 0.0 0.0 _returnvalue_yaw)) ActionValue)))

(event `EnhancedInput|/Game/TrollGame/Blueprints/Inputs/IA_MoveRight`
  (params (ActionValue :type "Float (double-precision)") (ElapsedSeconds :type "Float (double-precision)") (TriggeredSeconds :type "Float (double-precision)") (InputAction :type "InputAction Object Reference" :default "/Game/TrollGame/Blueprints/Inputs/IA_MoveRight.IA_MoveRight"))
  (bind (_returnvalue_roll _returnvalue_pitch _returnvalue_yaw) (`KismetMathLibrary.BreakRotator` (`self.GetControlRotation`)))
  ; Control de movimiento lateral
  (:`Triggered`
    (`self.AddMovementInput` (`KismetMathLibrary.GetRightVector` (`KismetMathLibrary.MakeRotator` 0.0 0.0 _returnvalue_yaw)) ActionValue)))

(event `self.ReceiveTick`
  (params (DeltaSeconds :type "Float (single-precision)"))
  (bind _camera (`self.Camera`))
  (bind _returnvalue (`SceneComponent.K2_GetComponentLocation` _camera))
  ; Check si golpea una pared via raycast
  (bind (_outhit _returnvalue_2) (`KismetSystemLibrary.LineTraceSingle` :`Start` _returnvalue :`End` (+ _returnvalue (* (`KismetMathLibrary.GetForwardVector` (`SceneComponent.K2_GetComponentRotation` _camera)) 600.0)) :`TraceChannel` "TraceTypeQuery1" :`DrawDebugType` "ForDuration"))
  (if _returnvalue_2
    (bind (_bblockinghit _binitialoverlap _time _distance _location _impactpoint _normal _impactnormal _physmat _hitactor) (`GameplayStatics.BreakHitResult` _outhit))
    ; si golpeo una pared verifica si es solida oh si es falsa
    (if (`KismetSystemLibrary.DoesImplementInterface` _hitactor "/Game/TrollGame/Blueprints/Interfaces/BPI_WallInteractions.BPI_WallInteractions_C")
      (bind _ewalltype (message `/Game/TrollGame/Blueprints/Interfaces/BPI_WallInteractions.GetWallType` _hitactor))
      (if (`|EnumEquality` _ewalltype "NewEnumerator0")
        (message `/Game/TrollGame/Blueprints/Interfaces/BPI_WallInteractions.ToggleWallState` _hitactor false)
        (else
          (message `/Game/TrollGame/Blueprints/Interfaces/BPI_WallInteractions.ToggleWallState` _hitactor true))))))

(fn `UserConstructionScript`)