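; BP_Wall_Fake is a troll wall whose collision is meant to alternate between solid and passable every eight seconds.
; A looping Delay from BeginPlay flips Solid and calls ToggleWallState with a fixed false argument.
; ToggleWallState branches on Solid values to set the Wall's collision profile to BlockAll or NoCollision.
; GetWallType separately maps the first actor tag, FakeWall or RealWall, to a wall-type enum, with a fallback value.
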(event `self.ReceiveBeginPlay`
  ; Mecanica troll cada 8 segundos la pared se vuelve solida
  (`KismetSystemLibrary.Delay` 8.0 :!label _label)
  (set `self.bSolid` (not (`self.bSolid`)))
  (`self.ToggleWallState` false)
  (goto _label))

(event `/Game/TrollGame/Blueprints/Interfaces/BPI_WallInteractions.ToggleWallState`
  (params (bSolid :type Boolean))
  (bind _wall (`self.Wall`))
  ; Hacer Pared Passable si es falsa
  (if (`self.bSolid`)
    (`PrimitiveComponent.SetCollisionProfileName` _wall "BlockAll" true :!label _label_2)
    (elif bSolid
      (goto _label_2)
      (else
        (`PrimitiveComponent.SetCollisionProfileName` _wall "NoCollision" true)))))

(fn `GetWallType`
  (returns (EWallType :type "/Game/TrollGame/Blueprints/Interfaces/Enum_WallType Enum"))
  (bind _output (`|GetArrayItem` (`self.Tags`)))
  ; Implementa el retorno del typo de pared via el tag de este
  (if (== _output "FakeWall")
    (return "NewEnumerator0")
    (elif (== _output "RealWall")
      (return "NewEnumerator1")
      (else
        (return "NewEnumerator3")))))

(fn `UserConstructionScript`)